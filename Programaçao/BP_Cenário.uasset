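; BP_Cenário is a self-chaining level segment for an endless side-scrolling stage.
; On BeginPlay it picks a random tile map, starts a timed self-destruct, and spawns a random obstacle or enemy and a random coin pickup at arrow components.
; When BP_Personagem overlaps its box, it spawns the next BP_Cenário at a fixed X offset from its tile map.
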(event `self.ReceiveBeginPlay`
  ;[1 1 1] Eventos
  (`self.Cenario Aleatorio`)
  (`self.Apagar Cenario`)
  (`self.Criar Obstaculo`)
  (`self.Criar Moedas`))

(event `self.Box.OnComponentBeginOverlap`
  (params (OverlappedComponent :type "PrimitiveComponent Object Reference") (OtherActor :type "Actor Object Reference") (OtherComp :type "PrimitiveComponent Object Reference") (OtherBodyIndex :type Integer) (bFromSweep :type Boolean) (SweepResult :type "HitResult Structure (by ref)"))
  (bind (_returnvalue_x _returnvalue_y _returnvalue_z) (`KismetMathLibrary.BreakVector` (`SceneComponent.K2_GetComponentLocation` (`self.PaperTileMap`))))
  ;[1 1 1] Mapas
  (cast `/Game/Programaçao/BP_Personagem` OtherActor)
  (`|SpawnActorFromClass` "BP_Cenário_C" (`KismetMathLibrary.MakeTransform` (`KismetMathLibrary.MakeVector` (+ _returnvalue_x 4086.0) _returnvalue_y _returnvalue_z)) "Undefined" "OverrideRootScale" null null))

(event `Cenario Aleatorio`
  ;[1 1 1] Cenario Aleatorio
  (`PaperTileMapComponent.SetTileMap` (`self.PaperTileMap`) (`|GetArrayItem` (`self.Cenario`) (`KismetMathLibrary.RandomIntegerInRange` 0 4))))

(event `Apagar Cenario`
  ;[1 1 1] Apagar Cenario
  (`KismetSystemLibrary.Delay` 20.0)
  (`self.K2_DestroyActor`))

(event `Criar Moedas`
  (bind _returnvalue (`SceneComponent.K2_GetComponentToWorld` (`self.Arrow Moeda`)))
  ;[1 0.9709 0.5724] Criar Moedas
  (switch `int` (`KismetMathLibrary.RandomIntegerInRange` 0 2)
    (:`0`
      (`|SpawnActorFromClass` "/Game/Programaçao/BP_Moeda.BP_Moeda_C" _returnvalue "Undefined" "OverrideRootScale" null null))
    (:`1`
      (`|SpawnActorFromClass` "/Game/Programaçao/BP_KitMoeda.BP_KitMoeda_C" _returnvalue "Undefined" "OverrideRootScale" null null))
    (:`2`
      (`|SpawnActorFromClass` "/Game/Programaçao/BP_KitMoeda2.BP_KitMoeda2_C" _returnvalue "Undefined" "OverrideRootScale" null null))))

(event `Criar Obstaculo`
  (bind _returnvalue (`SceneComponent.K2_GetComponentToWorld` (`self.Arrow`)))
  ;[1 1 1] Obstaculos
  (switch `int` (`KismetMathLibrary.RandomIntegerInRange` 0 2)
    (:`Default`
      (`|SpawnActorFromClass` "/Game/Programaçao/BP_ObsDestr.BP_ObsDestr_C" _returnvalue "Undefined" "OverrideRootScale" null null :!label _label))
    (:`0`
      (`|SpawnActorFromClass` "/Game/Programaçao/BP_Obstaculo.BP_Obstaculo_C" _returnvalue "Undefined" "OverrideRootScale" null null))
    (:`1`
      (goto _label))
    (:`2`
      (`|SpawnActorFromClass` "/Game/Programaçao/BP_Inimigo.BP_Inimigo_C" _returnvalue "Undefined" "OverrideRootScale" null null))))

(fn `UserConstructionScript`)