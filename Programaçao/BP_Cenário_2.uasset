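; BP_Cenário_2 is a self-destroying scenery segment that chains level pieces for continuous scrolling play.
; On BeginPlay it applies a random tile map from the Cenario array, spawns a BP_Obstaculo at its Arrow and starts a short timed self-destruct.
; When BP_Personagem overlaps its Box, it spawns a BP_Cenário at a fixed X offset from its tile map, extending the level ahead.
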(event `self.ReceiveBeginPlay`
  (`self.Cenario Aleatorio`)
  (`self.Apagar Cenario`)
  (`self.Criar Obstaculo`))

(event `self.Box.OnComponentBeginOverlap`
  (params (OverlappedComponent :type "PrimitiveComponent Object Reference") (OtherActor :type "Actor Object Reference") (OtherComp :type "PrimitiveComponent Object Reference") (OtherBodyIndex :type Integer) (bFromSweep :type Boolean) (SweepResult :type "HitResult Structure (by ref)"))
  (bind (_returnvalue_x _returnvalue_y _returnvalue_z) (`KismetMathLibrary.BreakVector` (`SceneComponent.K2_GetComponentLocation` (`self.PaperTileMap`))))
  (cast `/Game/Programaçao/BP_Personagem` OtherActor)
  (`|SpawnActorFromClass` "/Game/Programaçao/BP_Cenário.BP_Cenário_C" (`KismetMathLibrary.MakeTransform` (`KismetMathLibrary.MakeVector` (+ _returnvalue_x 4090.0) _returnvalue_y _returnvalue_z)) "Undefined" "OverrideRootScale" null null))

(event `Cenario Aleatorio`
  (`PaperTileMapComponent.SetTileMap` (`self.PaperTileMap`) (`|GetArrayItem` (`self.Cenario`) (`KismetMathLibrary.RandomIntegerInRange` 0 3))))

(event `Apagar Cenario`
  (`KismetSystemLibrary.Delay` 5.0)
  (`self.K2_DestroyActor`))

(event `Criar Obstaculo`
  (switch `int` (`KismetMathLibrary.RandomIntegerInRange` 0)
    (:`0`
      (`|SpawnActorFromClass` "/Game/Programaçao/BP_Obstaculo.BP_Obstaculo_C" (`SceneComponent.K2_GetComponentToWorld` (`self.Arrow`)) "Undefined" "OverrideRootScale" null null))))

(fn `UserConstructionScript`)