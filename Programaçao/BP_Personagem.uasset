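; BP_Personagem is the Paper2D player character of a side-scrolling auto-runner, jumping with Space and firing BP_Tiro with Enter.
; Tick moves it along +X, swaps run and jump flipbooks, locks camera height and checks for death.
; After a two-second grace period, near-zero velocity means death: the game pauses and shows WD_Derrota.
; BeginPlay also creates the HUD and starts a non-looping timer that slightly raises walk speed once.
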(event `self.ReceiveBeginPlay`
  ;[0.8818 0.5831 1] Begin Play
  (`self.Criar Interface`)
  (`self.Velocidade `)
  (`KismetSystemLibrary.Delay` 2.0)
  (set `self.Vulneravel` true))

(event `Andar`
  ;[1 0.6144 0.8613] Andar
  (if (not (`self.Morreu?`))
    (`self.AddMovementInput` (1.0 0.0 0.0))))

(event `self.ReceiveTick`
  (params (DeltaSeconds :type "Float (single-precision)"))
  ;[1 1 1] Event Tick
  (`self.Andar`)
  (`self.Atualizar Animação`)
  (`self.Travar Camera`)
  (`self.Conferir Morte`))

(event `Pulo`
  ;[1 0.6972 0.7171] Pular
  (if (not (`self.Morreu?`)) :!label _label
    (`self.Jump`)
    (`GameplayStatics.PlaySound2D` "/Game/Musica/8bit-jump__online-audio-converter_com_.8bit-jump__online-audio-converter_com_" 0.3 1.0 0.0 null null)))

(event `Travar Camera`
  (bind _camera (`self.Camera`))
  (bind (_returnvalue_x _returnvalue_y) (`KismetMathLibrary.BreakVector` (`SceneComponent.K2_GetComponentLocation` _camera)))
  ;[0.4393 1 0.6714] Câmera
  (`SceneComponent.K2_SetWorldLocation` _camera (`KismetMathLibrary.MakeVector` _returnvalue_x _returnvalue_y -850.0) false false))

(event `Key|SpaceBar`
  (params (Key :type "Key Structure"))
  ;[1 0.6972 0.7171] Pular
  (:`Pressed`
    (goto _label)))

(event `Velocidade`
  ;[0.8079 0.87 1] Velocidade
  (`KismetSystemLibrary.K2_SetTimerDelegate` (delegate `Aumentar`) 1.0))

(event `Atualizar Animação`
  ;[1 0.9468 0.6746] Animação
  (if (`self.Morreu?`)
    _
    (elif (`NavMovementComponent.IsFalling` (`self.CharacterMovement`))
      (`PaperFlipbookComponent.SetFlipbook` (`self.Sprite`) "/Game/Personagem/png/Jump_02.Jump_02")
      (else
        (`PaperFlipbookComponent.SetFlipbook` (`self.Sprite`) "/Game/Personagem/png/Run_02.Run_02")))))

(event `Aumentar`
  (bind _charactermovement (`self.CharacterMovement`))
  ;[0.8079 0.87 1] Velocidade
  (set `CharacterMovementComponent.MaxWalkSpeed` (+ (`CharacterMovementComponent.MaxWalkSpeed` _charactermovement) 1.0) _charactermovement))

(event `Conferir Morte`
  ;[0.4775 0.7954 1] Conferir Morte
  (if (`self.Vulneravel`)
    (if (<= (`KismetMathLibrary.VSize` (`MovementComponent.Velocity` (`self.CharacterMovement`))) 10.0)
      (set `self.Morreu?` true)
      (`PaperFlipbookComponent.SetFlipbook` (`self.Sprite`) "/Game/Personagem/png/Dead_02.Dead_02")
      (`GameplayStatics.SetGamePaused` true)
      (bind _returnvalue (`|CreateWidget` "/Game/Widget/WD_Derrota.WD_Derrota_C"))
      (`UserWidget.AddToViewport` _returnvalue 0))))

(event `Tiro`
  ;[0.8224 1 0.505] Tiro
  (if (not (`self.Morreu?`)) :!label _label_2
    (`|SpawnActorFromClass` "/Game/Programaçao/BP_Tiro.BP_Tiro_C" (`SceneComponent.K2_GetComponentToWorld` (`self.Arrow1`)) "Undefined" "OverrideRootScale" null null)
    (`GameplayStatics.PlaySound2D` "/Game/Musica/leftfoot8bit__online-audio-converter_com_.leftfoot8bit__online-audio-converter_com_" 0.5 1.0 0.0 null null)))

(event `Criar Interface`
  ;[0.9162 0.5487 1] Interface
  (bind _returnvalue (`|CreateWidget` "/Game/Widget/WD_Interface.WD_Interface_C"))
  (`UserWidget.AddToViewport` _returnvalue 0))

(event `Key|Enter`
  (params (Key :type "Key Structure"))
  ;[0.8224 1 0.505] Tiro
  (:`Pressed`
    (goto _label_2)))

(fn `UserConstructionScript`)